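; Round controller that runs data-table challenges as successive rounds of enemy groups and boxes.
; Construction caches spawn points and row names; selecting a challenge moves the player to the start and begins round one.
; Each round reveals enemy groups at random unused spawners and spawns boxes at random spawners, pruning the master box list.
; Emptying CurrentEnemies advances the round; after the last, it pays money and toggles the menu.
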(event Custom|NewRound
  (bind _player (Variables|Default|GetPlayer))
  (bind _currentchallenge (Variables|Default|GetCurrentChallenge))
  (bind _currentround (Variables|Default|GetCurrentRound))
  (bind (_moneypayout _induvidualround) (Utilities|Struct|BreakChallenge _currentchallenge))
  (bind _output (Utilities|Array|Get(acopy) _induvidualround _currentround))
  (bind (_groupofenemies _boxspawns) (Utilities|Struct|BreakInduvidualRound _output))
  ;[1 1 1] Spawn all enemies for a round
  ;;[1 1 1] Check if the last round was the final round
  (Class|PlayerHUD|UpdateHUDElements (Variables|/Script/UE4_RCArena.PlayerCharacter|GetHUDRef (Variables|Default|GetPlayer)) (Variables|Default|GetIn%20Args))
  (if (> (Variables|Default|GetCurrentRound) (- (Utilities|Array|Length _induvidualround) 1))
    ;;[1 1 1] End the challenge
    (Development|PrintString "Well Done!")
    (Utilities|FlowControl|Delay 5.0)
    (Class|PlayerCharacter|AddMoney _player _moneypayout)
    (Class|PlayerCharacter|ToggleMenu _player)
    (else
      (Variables|Challenge|SetAvailabeSpawns (Variables|Default|GetEnemySpawns))
      (Variables|Default|SetAvailableBoxSpawns (Variables|Default|GetBox%20Spawns))
      ;;[1 1 1] For each group of enemies, get a random, unused spawn point
      (for _array_element _groupofenemies
        (bind _output_get (Variables|Challenge|SetSpawnArrayIndex (Math|Random|RandomIntegerinRange 0 (- (Utilities|Array|Length (Variables|Challenge|GetAvailabeSpawns)) 1))))
        (Default|RevealSpawner (Utilities|Array|Get(acopy) (Variables|Challenge|GetAvailabeSpawns) _output_get) (.amountofenemy _array_element))
        (Utilities|Array|RemoveIndex (Variables|Challenge|GetAvailabeSpawns) (Variables|Challenge|GetSpawnArrayIndex)))
      (for _array_element_2 _boxspawns
        (for _index (range 0 (.amount _array_element_2))
          (bind _output_get_2 (Variables|Challenge|SetSpawnArrayIndex (Math|Random|RandomIntegerinRange 0 (- (Utilities|Array|Length (Variables|Default|GetAvailableBoxSpawns)) 1))))
          (Class|BoxSpawner|SpawnBox (Utilities|Array|Get(acopy) (Variables|Default|GetAvailableBoxSpawns) _output_get_2) (.type _array_element_2))
          (Utilities|Array|RemoveIndex (Variables|Default|GetBox%20Spawns) _output_get_2))))))

(event EventRemoveEnemyfromArray
  (params (InEnemy :type Base%20Enemy%20Object%20Reference))
  ;[1 1 1] Remove enemies from the CurrentEnemies array
  ;;[1 1 1] Find the in enemy in the CurrentEnemies array and remove it
  (Variables|Challenge|SetIn%20Enemy InEnemy)
  (for (_array_element _array_index) (Variables|Challenge|GetCurrentEnemies)
    (if (== _array_element (Variables|Challenge|GetIn%20Enemy))
      (Utilities|Array|RemoveIndex (Variables|Challenge|GetCurrentEnemies) _array_index)))
  ;;[1 1 1] Check if all enemies are dead (empty array).  If true, go to the next round
  (if (== (Utilities|Array|Length (Variables|Challenge|GetCurrentEnemies)) 0)
    (Math|Integer|IncrementInt (Variables|Default|GetCurrentRound)
      (:%20%20
        (CallFunction|NewRound)))))

(event EventSetCurrentChallenge
  (params (InChallengeIndex :type Integer))
  (bind _playerspawn (Variables|Default|GetPlayerSpawn))
  ;[1 1 1] Get the data table row with the provided index
  (bind _returnvalue (Utilities|GetDataTableRow (Variables|Default|GetFChallengeDataTable) (Utilities|Array|Get(acopy) (Variables|Challenge|GetChallengeRowNames) InChallengeIndex))
    (:then
      (Variables|Default|SetCurrentChallenge _returnvalue)
      (Variables|Default|SetCurrentRound 0)
      ;[1 1 1] Set player loc and rot to SpawnPoint
      (bind _outactors (Actor|GetAllActorsOfClass "/Game/Player/Blueprint/BP_PlayerCharacter.BP_PlayerCharacter_C"))
      (bind _output_get (Variables|Default|SetPlayer (Utilities|Array|Get(acopy) _outactors)))
      (Transformation|SetActorLocationAndRotation _output_get (Transformation|GetActorLocation _playerspawn) (Transformation|GetActorRotation _playerspawn))
      (CallFunction|NewRound))
    (:RowNotFound
      (Development|PrintString "None Found"))))

(fn ConstructionScript
  ;[1 1 1] Get the player spawn point
  (bind _outactors (Actor|GetAllActorsOfClass "/Game/Maps/ASSETS/BP_PlayerSpawnPoint.BP_PlayerSpawnPoint_C"))
  (Variables|Default|SetPlayerSpawn (Utilities|Array|Get(acopy) _outactors))
  ;[1 1 1] Get all EnemySpawns
  (bind _outactors_2 (Actor|GetAllActorsOfClass "/Game/Maps/ASSETS/BP_EnemySpawer.BP_EnemySpawer_C"))
  (Variables|Default|SetEnemySpawns _outactors_2)
  ;[1 1 1] Get all BoxSpawns
  (bind _outactors_3 (Actor|GetAllActorsOfClass "/Script/UE4_RCArena.BoxSpawner"))
  (Variables|Default|SetBox%20Spawns _outactors_3)
  ;[1 1 1] Set ChallengeRowNames
  (bind _outrownames (DataTable|GetDataTableRowNames (Variables|Default|GetFChallengeDataTable)))
  (Variables|Challenge|SetChallengeRowNames _outrownames))