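; Enemy spawner platform that rises out of the lava, spawns a group of enemies, then sinks back once they leave.
; A timeline lerps it 1000 units up from its origin, with a FlipFlop on finish alternating between spawning and marking it hidden.
; Enemies spawn across seven points in order and register with BP_RoundCtrl.
; End-overlap removes entries by matching class and reverses the timeline when none remain.
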(event Custom|Reveal%20Spawner
  (params (InEnemies :type Array%20of%20Amount%20Of%20Enemy%20Structures))
  (bind _origin (Variables|Default|GetOrigin))
  ;[1 1 1] Hide or reveal the spawner from the lava
  (bind _movementtimeline (Timeline|MovementTimeline PlayFromStart)
    (:Update
      (Transformation|SetActorLocation (Math|Vector|Lerp(Vector) _origin (+ _origin "0, 0,1000.000000") _movementtimeline) false false)
      (bind _outactors (Actor|GetAllActorsOfClass "/Game/Maps/ASSETS/BP_RoundCtrl.BP_RoundCtrl_C"))
      (Variables|Default|SetRound%20Control (Utilities|Array|Get(acopy) _outactors)))
    (:Finished
      (Utilities|FlowControl|FlipFlop
        (:A
          (Variables|Default|SetHidden? false)
          (CallFunction|SpawnEnemies InEnemies))
        (:B
          (Variables|Default|SetHidden? true))))))

(event Custom|Conceal%20Spawner
  (bind _origin (Variables|Default|GetOrigin))
  ;[1 1 1] Hide or reveal the spawner from the lava
  (bind _movementtimeline (Timeline|MovementTimeline ReverseFromEnd)
    (:Update
      (Transformation|SetActorLocation (Math|Vector|Lerp(Vector) _origin (+ _origin "0, 0,1000.000000") _movementtimeline) false false)
      (bind _outactors (Actor|GetAllActorsOfClass "/Game/Maps/ASSETS/BP_RoundCtrl.BP_RoundCtrl_C"))
      (Variables|Default|SetRound%20Control (Utilities|Array|Get(acopy) _outactors)))
    (:Finished
      (Utilities|FlowControl|FlipFlop
        (:A
          (Variables|Default|SetHidden? false)
          (CallFunction|SpawnEnemies (stale Custom|Reveal%20Spawner InEnemies)))
        (:B
          (Variables|Default|SetHidden? true))))))

(event Custom|SpawnEnemies
  (params (EnemiesToSpawn :type Array%20of%20Amount%20Of%20Enemy%20Structures))
  ;[1 1 1] Spawn provided group of enemies
  (Variables|Default|SetSpawnPoint 0)
  (Variables|Default|SetCurrentSpawnPointNo 0)
  (for _array_element EnemiesToSpawn
    (for _index (range 1 (.amount _array_element))
      (if (Utilities|ClassIsChildOf (.enemyclass _array_element) "/Script/UE4_RCArena.BaseEnemy")
        ;;[1 1 1] Set the enemy class
        (Variables|Default|SetEnemy%20Class (.enemyclass _array_element))
        ;;[1 1 1] Get the spawn point to use
        (switch int (Variables|Default|GetCurrentSpawnPointNo)
          (:0
            (Variables|Default|SetSpawnPoint (Variables|Default|GetSpawnPoint1)))
          (:1
            (Variables|Default|SetSpawnPoint (Variables|Default|GetSpawnPoint2)))
          (:2
            (Variables|Default|SetSpawnPoint (Variables|Default|GetSpawnPoint3)))
          (:3
            (Variables|Default|SetSpawnPoint (Variables|Default|GetSpawnPoint4)))
          (:4
            (Variables|Default|SetSpawnPoint (Variables|Default|GetSpawnPoint5)))
          (:5
            (Variables|Default|SetSpawnPoint (Variables|Default|GetSpawnPoint6)))
          (:6
            (Variables|Default|SetSpawnPoint (Variables|Default|GetSpawnPoint7))))
        ;;[1 1 1] Spawn Enemy
        (bind _returnvalue (Game|SpawnActorfromClass (Variables|Default|GetEnemy%20Class) (Math|Transform|MakeTransform (Transformation|GetWorldLocation (Variables|Default|GetSpawnPoint)) (Transformation|GetWorldRotation (Variables|Default|GetSpawnPoint))) "AlwaysSpawn" 0 0))
        (Math|Integer|IncrementInt (Variables|Default|GetCurrentSpawnPointNo)
          (:%20%20
            (Utilities|Array|Add (Variables|Default|GetEnemiesArray) _returnvalue)
            (bind _asbase_enemy (Utilities|Casting|CastToBaseEnemy _returnvalue))
            (Utilities|Array|Add (Variables|/Game/Maps/ASSETS/BP_RoundCtrl.BP_RoundCtrl_C|GetCurrentEnemies (Variables|Default|GetRound%20Control)) _asbase_enemy)))))))

(event Collision|EventActorEndOverlap
  (params (OtherActor :type Actor%20Object%20Reference))
  (bind _enemiesarray (Variables|Default|GetEnemiesArray))
  ;[1 1 1] Remove the enemy that moved off the platform from the array.  If they are the last one, conceal the spawner
  (for (_array_element _array_index) (Variables|Default|GetEnemiesArray)
    (if (== (Utilities|GetClass _array_element) (Utilities|GetClass OtherActor))
      (Utilities|Array|RemoveIndex _enemiesarray _array_index)
      (if (== (Utilities|Array|Length _enemiesarray) 0)
        (CallFunction|ConcealSpawner)))))

(event EventBeginPlay
  ;[1 1 1] Set the world location
  (Variables|Default|SetOrigin (Transformation|GetWorldLocation (Variables|Default|GetDefaultSceneRoot))))

(fn ConstructionScript)