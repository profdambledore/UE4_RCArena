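; BP_Lava is a lava hazard that bounces the player on contact and kills them after repeated touches.
; Its Box overlap responds only to actors whose class is exactly BP_PlayerCharacter.
; The touch count lives on the player and is compared with MaxTimesTouchLava; reaching it calls KillPlayer.
; Earlier touches call SetInvunrabilityTime for damage, increment the count, print a debug message and trigger Jump.
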(event OnComponentBeginOverlap(Box)
  (params (OverlappedComponent :type Primitive%20Component%20Object%20Reference) (OtherActor :type Actor%20Object%20Reference) (OtherComp :type Primitive%20Component%20Object%20Reference) (OtherBodyIndex :type Integer) (bFromSweep :type Boolean) (SweepResult :type Hit%20Result%20Structure%20%28by%20ref%29))
  ;[1 1 1] Check if the PlayerCharacter is the one which collided with the Lava
  (if (== (Utilities|GetClass OtherActor) "/Game/Player/Blueprint/BP_PlayerCharacter.BP_PlayerCharacter_C")
    ;[1 1 1] Check if the player has touched the lava multiple times
    (bind _asbp_player_character (Utilities|Casting|CastToBP_PlayerCharacter OtherActor))
    (Variables|Default|SetAs%20BP%20Player%20Character _asbp_player_character)
    (if (== (+ (Variables|/Script/UE4_RCArena.PlayerCharacter|GetTimesTouchedLava _asbp_player_character) 1) (Variables|Default|GetMaxTimesTouchLava))
      (Class|PlayerCharacter|KillPlayer (Variables|Default|GetAs%20BP%20Player%20Character))
      (else
        ;[1 1 1] Make them take damage and launch them upwards
        (Class|PlayerCharacter|SetInvunrabilityTime (Variables|Default|GetAs%20BP%20Player%20Character) 0.1 1)
        (Math|Integer|IncrementInt (Variables|/Script/UE4_RCArena.PlayerCharacter|GetTimesTouchedLava (Variables|Default|GetAs%20BP%20Player%20Character))
          (:%20%20
            (Development|PrintString "Touched Lava")
            (Character|Jump (Variables|Default|GetAs%20BP%20Player%20Character))))))))

(fn ConstructionScript)