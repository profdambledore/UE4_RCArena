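; BP_MoneyPickup is a pickup that takes on a random money appearance and amount.
; On BeginPlay it picks a random index into the MoneyTypes array, then sets Amount and the PickupMesh static mesh from that entry.
; If the last entry is chosen, PickupMeshAdd also receives SM_MoneyTiny2 as the second part of that mesh.
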(event EventBeginPlay
  ;[1 1 1] Set the mesh(es)
  ;;[1 1 1] Get the mesh from the array and set the amount
  (bind _output_get (Variables|Default|Seti (Math|Random|RandomIntegerinRange 0 (- (Utilities|Array|Length (Variables|Default|GetMoneyTypes)) 1))))
  (Variables|Default|SetAmount (.amount (Utilities|Array|Get(acopy) (Variables|Default|GetMoneyTypes) _output_get)))
  (Components|StaticMesh|SetStaticMesh (Variables|Default|GetPickupMesh) (.mesh (Utilities|Array|Get(acopy) (Variables|Default|GetMoneyTypes) _output_get)))
  ;;[1 1 1] Check to see if the index chosen is the last.  If it is, set the mesh add to the secone part of the mesh
  (if (== (Variables|Default|Geti) (- (Utilities|Array|Length (Variables|Default|GetMoneyTypes)) 1))
    (Components|StaticMesh|SetStaticMesh (Variables|Default|GetPickup%20Mesh%20Add) "/Game/Pickup/Mesh/SM_MoneyTiny2.SM_MoneyTiny2")))

(fn ConstructionScript)