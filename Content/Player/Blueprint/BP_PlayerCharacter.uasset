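; BP_PlayerCharacter is the player character Blueprint and handles multi-jump input.
; Pressing Jump increments a jump counter, calls Jump and sets an in-air flag while the count is below MaxJumps, with a debug print.
; Releasing the input stops jumping, and landing clears the flag and resets the counter.
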(event EventOnLanded
  (params (Hit :type Hit%20Result%20Structure%20%28by%20ref%29))
  ;[1 1 1] Jumping
  (Variables|Default|SetbInAir false)
  (Variables|Default|SetCurrJumps 0))

(event Input|ActionEvents|InputActionJump
  (params (Key :type Key%20Structure :default "None"))
  (bind _currjumps (Variables|Default|GetCurrJumps))
  ;[1 1 1] Jumping
  (:Pressed
    (if (< _currjumps (Variables|Default|GetMaxJumps))
      (Math|Integer|IncrementInt _currjumps
        (:%20%20
          (Character|Jump)
          (Variables|Default|SetbInAir true)
          (Development|PrintString "Hello")))))
  (:Released
    (Character|StopJumping)))

(fn ConstructionScript)